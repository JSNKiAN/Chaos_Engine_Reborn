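; BP_Duelist_P2 is the second duelist, which acts as a CPU opponent when IsPlayer2 is false.
; It sends itself to BP_Camera through BPI_Player_Track on BeginPlay and again every Tick.
; In CPU mode it chases player one with AI MoveTo, reissued on success and by a repeating delay loop.
; BeginPlay also creates an on-screen health bar bound to this duelist, unless the CPU loop precedes it indefinitely.
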(event `self.ReceiveBeginPlay`
  (`|ExecutionSequence`
    (:`then_0`
      ;[0.05098 0.05098 0.05098] Begin Get Player Two Ref > BPI_Player_Track
      (bind _returnvalue (`GameplayStatics.GetActorOfClass` "/Game/Blueprints/Camera/BP_Camera.BP_Camera_C"))
      (message `/Game/Blueprints/Camera/BPI_PlayerTrack.PlayerTwoRef` _returnvalue self)
      ;[0.05098 0.05098 0.05098] CPU or Player 2
      (if (not (`self.IsPlayer2?`))
        ;[0.05098 0.05098 0.05098] Loop CPU Follow Player Function
        (`self.Follow Player` :!label _label)
        (`KismetSystemLibrary.Delay` 2.0)
        (goto _label)))
    (:`then_1`
      (bind _returnvalue_2 (`|CreateWidget` "/Game/DamageSystem/WB_Duelist_HealthBar.WB_Duelist_HealthBar_C" null self))
      (`UserWidget.AddToViewport` _returnvalue_2 0))))

(event `Follow Player`
  ;[0.05098 0.05098 0.05098] Follow Player One
  (`|AIMoveTo` self (0.0 0.0 0.0) (`GameplayStatics.GetPlayerCharacter` 0) 100.0
    (:`OnSuccess`
      (`self.Follow Player`))))

(event `self.ReceiveTick`
  (params (DeltaSeconds :type "Float (single-precision)"))
  ;[0.05098 0.05098 0.05098] Update Player Two Ref > BPI_Player_Track
  (bind _returnvalue (`GameplayStatics.GetActorOfClass` "/Game/Blueprints/Camera/BP_Camera.BP_Camera_C"))
  (message `/Game/Blueprints/Camera/BPI_PlayerTrack.PlayerTwoRef` _returnvalue self))

(fn `UserConstructionScript`
  (`parent.UserConstructionScript`))