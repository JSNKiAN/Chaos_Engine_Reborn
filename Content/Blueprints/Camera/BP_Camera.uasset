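; Shared top-down camera actor that follows two players, or only player one in a test mode.
; A game mode setup binding makes it player 0's view target, and incoming player references move it to the pair's midpoint.
; Tick eases spring arm yaw toward a target changed in steps by turn events, sets arm length from clamped player distance, and sends the arm to controllers.
; Turn-stop events retain older timeline-driven free rotation.
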(event `self.ReceiveBeginPlay`
  ;[0.05098 0.05098 0.05098] Begin Play (Init)
  (bind _asbp_top_down_game_mode (cast `/Game/Blueprints/BP_TopDownGameMode` (`GameplayStatics.GetGameMode`)))
  (add `/Game/Blueprints/BP_TopDownGameMode.SetUpCamera` _asbp_top_down_game_mode (`|CreateDelegate` :!event `Init`)))

(event `Init`
  ;[0.05098 0.05098 0.05098] Sets Player Character's Camera to current actor
  (`KismetSystemLibrary.Delay` 0.01)
  (`PlayerController.SetViewTargetWithBlend` (`GameplayStatics.GetPlayerController` 0) self 0.0 "VTBlend_Linear" 0.0 false)
  (bind _outactors (`GameplayStatics.GetAllActorsOfClass` "/Game/Blueprints/Player/BP_TopDownCharacter.BP_TopDownCharacter_C"))
  (set `self.Players` _outactors)
  (`self.SetActorTickEnabled` true))

(event `/Game/Blueprints/Camera/BPI_TurnCamera.TurnRStart`
  ;[0.05098 0.05098 0.05098] 90° Rotation
  (set `self.NewCameraVector` (+ (`self.NewCameraVector`) (`KismetMathLibrary.MakeVector` 0.0 0.0 (`self.RotationAmount`)))))

(event `self.ReceiveTick`
  (params (DeltaSeconds :type "Float (single-precision)"))
  (bind (_newcameravector_x _newcameravector_y _newcameravector_z) (`KismetMathLibrary.BreakVector` (`self.NewCameraVector`)))
  (bind (_returnvalue_roll _returnvalue_pitch _returnvalue_yaw) (`KismetMathLibrary.BreakRotator` (`SpringArmComponent.GetTargetRotation` (`self.SpringArm`))))
  (set `self.DeltaSeconds` DeltaSeconds)
  (`SceneComponent.K2_SetWorldRotation` (`self.SpringArm`) (`KismetMathLibrary.RInterpTo` (`KismetMathLibrary.MakeRotator` _returnvalue_roll _returnvalue_pitch _returnvalue_yaw) (`KismetMathLibrary.MakeRotator` _returnvalue_roll _returnvalue_pitch _newcameravector_z) (`self.DeltaSeconds`) (`self.RotationSpeed`)) false false)
  ;[0.05098 0.05098 0.05098] Send Spring Arm Vector to Controller
  (bind _outactors (`GameplayStatics.GetAllActorsOfClass` "/Game/Blueprints/BP_TopDownController.BP_TopDownController_C"))
  (message `/Game/Blueprints/Camera/BPI_TurnCamera.SpringArmRef` _outactors (`self.SpringArm`))
  (set `SpringArmComponent.TargetArmLength` (`KismetMathLibrary.FClamp` (* (`self.GetDistanceTo` (`self.Player One Ref`) (`self.Player Two Ref`)) 1.0) 900.0 1400.0) (`self.SpringArm`)))

(event `/Game/Blueprints/Camera/BPI_TurnCamera.TurnLStart`
  ;[0.05098 0.05098 0.05098] 90° Rotation
  (set `self.NewCameraVector` (+ (`self.NewCameraVector`) (`KismetMathLibrary.MakeVector` 0.0 0.0 (* (`self.RotationAmount`) -1.0)))))

(event `/Game/Blueprints/Camera/BPI_TurnCamera.TurnRStop`
  ;[0.05098 0.05098 0.05098] Free Rotation (Old)
  (bind (_direction _0_to_2) (`Timeline|Timeline_1` :!via `Reverse`)
    (:`Update`
      (`SceneComponent.K2_AddWorldRotation` (`self.SpringArm`) (`KismetMathLibrary.MakeRotator` 0.0 0.0 _0_to_2) false false))))

(event `/Game/Blueprints/Camera/BPI_TurnCamera.TurnLStop`
  ;[0.05098 0.05098 0.05098] Free Rotation (Old)
  (bind (_direction _0_to_2) (`Timeline|Timeline` :!via `Reverse`)
    (:`Update`
      (`SceneComponent.K2_AddWorldRotation` (`self.SpringArm`) (`KismetMathLibrary.MakeRotator` 0.0 0.0 (* _0_to_2 -1.0)) false false))))

(event `/Game/Blueprints/Camera/BPI_PlayerTrack.PlayerOneRef`
  (params (PlayerOneRef :type "Actor Object Reference"))
  ;[0.05098 0.05098 0.05098] Get Player Vector & Follow
  ;;[0.05098 0.05098 0.05098] Follow One Player
  (bind _output_get (set `self.Player One Ref` PlayerOneRef))
  (`self.Player Two Ref`
    (:`then`
      (if (`self.OnlyPlayerOneTest`)
        (bind _returnvalue (`self.K2_GetActorLocation` _output_get))
        (`self.K2_SetActorTransform` self (`KismetMathLibrary.Conv_VectorToTransform` _returnvalue) false false)
        (else
          ;;[0.05098 0.05098 0.05098] Follow Two Players
          (`self.K2_SetActorTransform` self (`KismetMathLibrary.Conv_VectorToTransform` (`KismetMathLibrary.VLerp` _returnvalue (`self.K2_GetActorLocation` (stale `/Game/Blueprints/Camera/BPI_PlayerTrack.PlayerTwoRef` _output_get)) 0.5)) false false))))
    (:`else`)))

(event `/Game/Blueprints/Camera/BPI_PlayerTrack.PlayerTwoRef`
  (params (PlayerTwoRef :type "Actor Object Reference"))
  ;[0.05098 0.05098 0.05098] Get Player Vector & Follow
  ;;[0.05098 0.05098 0.05098] Follow Two Players
  (bind _output_get (set `self.Player Two Ref` PlayerTwoRef)))

(fn `UserConstructionScript`)