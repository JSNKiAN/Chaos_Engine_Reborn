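; Wrecking ball projectile that damages either of the first two players on sphere overlap, then destroys itself.
; On BeginPlay, a timeline pushes the ball with force along the actor's initial forward vector.
; After a three-second delay, a second timeline scales the actor down and destroys it when finished.
; Damage goes through a TakeDamage message to the sweep's hit actor; its own health and damage functions are empty stubs.
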(event `self.ReceiveBeginPlay`
  (`|ExecutionSequence`
    (:`then_0`
      (set `self.EnemyForwardVector` (`self.GetActorForwardVector`))
      (`Timeline|Timeline_0`
        (:`Update`
          (`PrimitiveComponent.AddForce` (`self.Wrecking_Balls`) (* (`self.EnemyForwardVector`) 100000.0) "None" false))))
    (:`then_1`
      (`KismetSystemLibrary.Delay` 3.0)
      (bind (_direction _1_to_0) (`Timeline|Timeline`)
        (:`Update`
          (`self.SetActorScale3D` (`KismetMathLibrary.Conv_DoubleToVector` _1_to_0)))
        (:`Finished`
          (`self.K2_DestroyActor`))))))

(event `self.Sphere.OnComponentBeginOverlap`
  (params (OverlappedComponent :type "PrimitiveComponent Object Reference") (OtherActor :type "Actor Object Reference") (OtherComp :type "PrimitiveComponent Object Reference") (OtherBodyIndex :type Integer) (bFromSweep :type Boolean) (SweepResult :type "HitResult Structure (by ref)"))
  (`|ExecutionSequence`
    (:`then_0`
      (if (== (`GameplayStatics.GetPlayerPawn` 0) OtherActor)
        (message `/Game/DamageSystem/BPI_Damagable.TakeDamage` (`.HitActor` (`GameplayStatics.BreakHitResult` SweepResult)) (make `/Game/DamageSystem/S_DamageInfo` 10.0 "NewEnumerator2" "NewEnumerator1"))
        (`self.K2_DestroyActor` :!label _label)))
    (:`then_1`
      (if (== (`GameplayStatics.GetPlayerPawn` 1) OtherActor)
        (message `/Game/DamageSystem/BPI_Damagable.TakeDamage` (`.HitActor` (`GameplayStatics.BreakHitResult` SweepResult)) (make `/Game/DamageSystem/S_DamageInfo` 10.0 "NewEnumerator2" "NewEnumerator1"))
        (goto _label)))))

(fn `GetCurrentHealth`
  (returns (Health :type "Float (double-precision)"))
  (return 0.0))

(fn `GetMaxHealth`
  (returns (MaxHealth :type "Float (double-precision)"))
  (return 0.0))

(fn `Heal`
  (params (Amount :type "Float (double-precision)"))
  (returns (NewHealth :type "Float (double-precision)"))
  (return 0.0))

(fn `TakeDamage`
  (params (DamageInfo :type "/Game/DamageSystem/S_DamageInfo Structure"))
  (returns (WasDamaged :type Boolean))
  (return false))

(fn `UserConstructionScript`)