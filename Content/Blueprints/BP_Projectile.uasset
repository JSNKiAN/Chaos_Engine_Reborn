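; Projectile actor that fires with sound and particles, ignores both player pawns when moving, and destroys itself after a lifetime timer.
; Construction script applies Speed to its movement component; the Gravity assignment is unconnected.
; Sphere hits, or overlaps with the first-found Hand or Big Man enemy AI, broadcast OnProjectileImpact, play impact effects and destroy it.
; Health and damage functions are stubs returning zero or false.
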(event `self.ReceiveBeginPlay`
  (bind _returnvalue (`self.K2_GetActorLocation`))
  ;[0.05098 0.05098 0.05098] Ignore Player Actor Collision
  (`PrimitiveComponent.IgnoreActorWhenMoving` (`self.SphereCollision`) (`GameplayStatics.GetPlayerPawn` 0) true)
  (`PrimitiveComponent.IgnoreActorWhenMoving` (`self.SphereCollision`) (`GameplayStatics.GetPlayerPawn` 1) true)
  ;[0.05098 0.05098 0.05098] Play Sound & Effect on Fire
  (`GameplayStatics.PlaySoundAtLocation` (`self.ShootSound`) _returnvalue (struct) (`self.Volume Multiplier`) 1.0 0.0 null null null null)
  (`GameplayStatics.SpawnEmitterAtLocation` (`self.Shoot Effect`) _returnvalue)
  ;[0.05098 0.05098 0.05098] Projectile Lifetimer
  (`KismetSystemLibrary.K2_SetTimerDelegate` (delegate `ProjectileLife`) (`self.LifeTimer`)))

(event `ProjectileLife`
  ;[0.05098 0.05098 0.05098] Projectile Lifetimer
  (`self.K2_DestroyActor`))

(event `self.SphereCollision.OnComponentHit`
  (params (HitComponent :type "PrimitiveComponent Object Reference") (OtherActor :type "Actor Object Reference") (OtherComp :type "PrimitiveComponent Object Reference") (NormalImpulse :type "Vector Structure") (Hit :type "HitResult Structure (by ref)"))
  (bind (_bblockinghit _binitialoverlap _time _distance _location) (`GameplayStatics.BreakHitResult` Hit))
  ;[0.05098 0.05098 0.05098] Play Sound & Effect on Impact
  (`self.OnProjectileImpact` OtherActor Hit)
  (`GameplayStatics.SpawnEmitterAtLocation` (`self.ImpactEffect`) _location :!label _label)
  (`GameplayStatics.PlaySoundAtLocation` (`self.ImpactSound`) _location (struct) (`self.Volume Multiplier`) 1.0 0.0 null null null null)
  (`self.K2_DestroyActor`))

(event `self.SphereCollision.OnComponentBeginOverlap`
  (params (OverlappedComponent :type "PrimitiveComponent Object Reference") (OtherActor :type "Actor Object Reference") (OtherComp :type "PrimitiveComponent Object Reference") (OtherBodyIndex :type Integer) (bFromSweep :type Boolean) (SweepResult :type "HitResult Structure (by ref)"))
  (`|ExecutionSequence`
    (:`then_0`
      (bind _returnvalue (`GameplayStatics.GetActorOfClass` "/Game/Blueprints/Enemy/BP_Hand_EnemyAI.BP_Hand_EnemyAI_C"))
      (if (== _returnvalue OtherActor)
        (`self.OnProjectileImpact` _returnvalue SweepResult)
        (goto _label)))
    (:`then_1`
      (bind _returnvalue_2 (`GameplayStatics.GetActorOfClass` "/Game/Blueprints/Enemy/BP_Big_Man_EnemyAI.BP_Big_Man_EnemyAI_C"))
      (if (== _returnvalue_2 OtherActor)
        (`self.OnProjectileImpact` _returnvalue_2 SweepResult)
        (goto _label)))))

(fn `GetCurrentHealth`
  (returns (Health :type "Float (double-precision)"))
  (return 0.0))

(fn `GetMaxHealth`
  (returns (MaxHealth :type "Float (double-precision)"))
  (return 0.0))

(fn `Heal`
  (params (Amount :type "Float (double-precision)"))
  (returns (NewHealth :type "Float (double-precision)"))
  (return 0.0))

(fn `TakeDamage`
  (params (DamageInfo :type "/Game/DamageSystem/S_DamageInfo Structure"))
  (returns (WasDamaged :type Boolean))
  (return false))

(fn `UserConstructionScript`
  (bind _projectilemovement (`self.ProjectileMovement`))
  (bind _speed (`self.Speed`))
  (set `ProjectileMovementComponent.InitialSpeed` _speed _projectilemovement)
  (set `ProjectileMovementComponent.MaxSpeed` _speed _projectilemovement))